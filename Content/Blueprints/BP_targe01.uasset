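; BP_targe01 is a shootable target actor that awards score when it takes damage.
; On AnyDamage, only the server casts the instigator's PlayerState to MyPlayerState and calls IncrementScore.
; A timeline graph for moving the Cube along a Spline is present but never runs.
; That unused movement feeds local-space spline positions into SetWorldLocation.
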(event `self.ReceiveAnyDamage`
  (params (Damage :type "Float (single-precision)") (DamageType :type "DamageType Object Reference") (InstigatedBy :type "Controller Object Reference") (DamageCauser :type "Actor Object Reference"))
  ;[1 1 1] 击中物体加分
  (`/Engine/EditorBlueprintResources/ActorMacros.Switch Has Authority`
    (:`Authority`
      (bind _asmy_player_state (cast `/Game/Blueprints/MyPlayerState` (`Controller.PlayerState` InstigatedBy)))
      (`/Game/Blueprints/MyPlayerState.IncrementScore` _asmy_player_state))))

(fn `UserConstructionScript`)