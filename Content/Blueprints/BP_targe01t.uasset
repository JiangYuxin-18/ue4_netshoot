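; BP_targe01t is a target actor that awards score to the player who damages it.
; On AnyDamage, the authority casts the instigator's PlayerState to MyPlayerState and calls IncrementScore.
; A timeline meant to move the Cube along a Spline is present but never runs, and it feeds local-space spline positions into SetWorldLocation.
; The Cube hit event and construction script are empty.
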(event `self.ReceiveAnyDamage`
  (params (Damage :type "Float (single-precision)") (DamageType :type "DamageType Object Reference") (InstigatedBy :type "Controller Object Reference") (DamageCauser :type "Actor Object Reference"))
  ;[1 1 1] 击中物体加分
  (`/Engine/EditorBlueprintResources/ActorMacros.Switch Has Authority`
    (:`Authority`
      (bind _asmy_player_state (cast `/Game/Blueprints/MyPlayerState` (`Controller.PlayerState` InstigatedBy)))
      (`/Game/Blueprints/MyPlayerState.IncrementScore` _asmy_player_state))))

(event `self.Cube.OnComponentHit`
  (params (HitComponent :type "PrimitiveComponent Object Reference") (OtherActor :type "Actor Object Reference") (OtherComp :type "PrimitiveComponent Object Reference") (NormalImpulse :type "Vector Structure") (Hit :type "HitResult Structure (by ref)")))

(fn `UserConstructionScript`)